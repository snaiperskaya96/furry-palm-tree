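; Behavior tree task that picks the nearest player pawn as the AI's target.
; On execute, it loops over the game state's player array and keeps the valid pawn closest to the controlled pawn, starting from any previously stored closest player.
; It writes that pawn to the "Target" blackboard key, hard-coded by name, and succeeds only if a valid target exists.
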(event `self.ReceiveExecuteAI`
  (params (OwnerController :type "AIController Object Reference") (ControlledPawn :type "Pawn Object Reference"))
  (bind _closestplayer (`self.ClosestPlayer`))
  (bind _closestplayer_2 (`self.ClosestPlayer`))
  (for _array_element (`GameStateBase.PlayerArray` (`GameplayStatics.GetGameState`))
    (bind _pawnprivate (`PlayerState.PawnPrivate` _array_element))
    (`/Engine/EditorBlueprintResources/StandardMacros.IsValid` _pawnprivate
      (:`Is Valid`
        (`/Engine/EditorBlueprintResources/StandardMacros.IsValid` _closestplayer
          (:`Is Valid`
            (if (< (`Actor.GetDistanceTo` ControlledPawn _pawnprivate) (`Actor.GetDistanceTo` ControlledPawn _closestplayer))
              (set `self.ClosestPlayer` _pawnprivate)))
          (:`Is Not Valid`
            (set `self.ClosestPlayer` _pawnprivate))))))
  (`BTFunctionLibrary.SetBlackboardValueAsObject` (make `BlackboardKeySelector` :`SelectedKeyName` "Target" :`SelectedKeyType` "/Script/AIModule.BlackboardKeyType_Object" :`bNoneIsAllowedValue` true) _closestplayer_2)
  (`self.FinishExecute` (`KismetSystemLibrary.IsValid` _closestplayer_2)))