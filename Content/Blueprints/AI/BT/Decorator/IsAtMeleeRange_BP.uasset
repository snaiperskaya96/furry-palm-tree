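; Behavior tree decorator that passes when the AI pawn is within melee range of its blackboard target.
; It line-traces against Pawn objects from the target to the controlled pawn, ignoring the target, with a one-frame debug draw.
; The check succeeds only if the first hit is the controlled pawn and its distance is within MaxDistance, so another pawn in between blocks it.
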(fn `PerformConditionCheck`
  (params (OwnerActor :type "Actor Object Reference"))
  (returns (ReturnValue :type Boolean))
  (locals (TargetKeyName :type Name :default "Target")))

(fn `PerformConditionCheckAI`
  (params (OwnerController :type "AIController Object Reference") (ControlledPawn :type "Pawn Object Reference"))
  (returns (ReturnValue :type Boolean))
  (locals (TargetKeyName :type Name :default "Target"))
  (bind _asactor (cast `Actor` (`BlackboardComponent.GetValueAsObject` (`AIBlueprintHelperLibrary.GetBlackboard` ControlledPawn) (`local.TargetKeyName`))))
  (bind (_outhit _returnvalue) (`KismetSystemLibrary.LineTraceSingleForObjects` (`Actor.K2_GetActorLocation` _asactor) (`Actor.K2_GetActorLocation` ControlledPawn) (`|MakeArray` "ObjectTypeQuery3" :!type "EObjectTypeQuery Enum") false (`|MakeArray` _asactor) "ForOneFrame"))
  (if _returnvalue
    (return (and (<= (`.Distance` (`GameplayStatics.BreakHitResult` _outhit)) (`self.MaxDistance`)) (== (`.HitActor` (`GameplayStatics.BreakHitResult` _outhit)) ControlledPawn)))
    (else
      (return false))))