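; Behavior tree decorator that gates AI branches on whether the agent has a controlled Pawn as its target.
; It reads the object stored under TargetKeyName from the owner's Blackboard.
; The check passes only when that object is valid, casts to Pawn and has a valid Controller, so an unpossessed Pawn does not count as a target.
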(fn `PerformConditionCheck`
  (params (OwnerActor :type "Actor Object Reference"))
  (returns (ReturnValue :type Boolean))
  (locals (TargetKeyName :type Name :default "Target"))
  (bind _returnvalue (`BlackboardComponent.GetValueAsObject` (`AIBlueprintHelperLibrary.GetBlackboard` OwnerActor) (`local.TargetKeyName`)))
  (bind (_aspawn _bsuccess) (cast `Pawn` _returnvalue :!pure true))
  (if (`KismetSystemLibrary.IsValid` _returnvalue)
    (return (and _bsuccess (`KismetSystemLibrary.IsValid` (`Pawn.GetController` _aspawn))))
    (else
      (return false))))