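; PimpMyGunStation is a weapon customization station that displays a rotating M4 and shows an interaction prompt on overlap.
; Interact stops the rotation and opens the PimpMyGun widget in UI-only input mode, passing itself as the Station.
; Save equips a clone of the display weapon on the player character.
; Save and Cancel both recreate the display M4, resume rotation, restore game input and blend the view back to the player.
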(event `self.ReceiveBeginPlay`
  (`self.RecreateWeapon`))

(event `self.ReceiveTick`
  (params (DeltaSeconds :type "Float (single-precision)"))
  (if (`self.ShouldRotate`)
    (`SceneComponent.K2_AddLocalRotation` (`self.Scene`) (struct :`Yaw` 1.0) false false)))

(event `self.ReceiveActorBeginOverlap`
  (params (OtherActor :type "Actor Object Reference"))
  (bind _returnvalue (`|CreateWidget` "/Game/Blueprints/PimpMyGun/PimpMyGunInteractionWidget.PimpMyGunInteractionWidget_C"))
  (bind _output_get (set `self.InteractionWidget` _returnvalue))
  (`UserWidget.AddToViewport` _output_get 0))

(event `self.ReceiveActorEndOverlap`
  (params (OtherActor :type "Actor Object Reference"))
  (bind _interactionwidget (`self.InteractionWidget`))
  (`Widget.RemoveFromParent` _interactionwidget)
  (`Widget.SetVisibility` _interactionwidget "Collapsed"))

(fn `Cancel`
  (`self.Quit`))

(fn `Interact`
  (bind _returnvalue (`GameplayStatics.GetPlayerController` 0))
  (set `self.ShouldRotate` false)
  (`SceneComponent.K2_SetRelativeRotation` :`self` (`self.Scene`))
  (bind _returnvalue_2 (`|CreateWidget` "/Game/Blueprints/PimpMyGun/PimpMyGun.PimpMyGun_C" _returnvalue self))
  (bind _output_get (set `self.PimpMyGunWidget` _returnvalue_2))
  (`UserWidget.AddToViewport` _output_get 0)
  (`WidgetBlueprintLibrary.SetInputMode_UIOnlyEx` _returnvalue _output_get)
  (`Widget.SetVisibility` (`self.InteractionWidget`) "Collapsed")
  (set `PlayerController.bShowMouseCursor` true _returnvalue))

(fn `OnAccessoryChanged`)

(fn `Quit`
  (bind _returnvalue (`GameplayStatics.GetPlayerController` 0))
  (bind _pimpmygunwidget (`self.PimpMyGunWidget`))
  (`self.RecreateWeapon`)
  (set `self.ShouldRotate` true)
  (`Widget.RemoveFromParent` _pimpmygunwidget)
  (`Widget.SetVisibility` _pimpmygunwidget "Collapsed")
  (`Widget.SetVisibility` (`self.InteractionWidget`) "HitTestInvisible")
  (`PlayerController.SetViewTargetWithBlend` _returnvalue (`GameplayStatics.GetPlayerCharacter` 0) 1.0 "VTBlend_Linear" 0.0 false)
  (`WidgetBlueprintLibrary.SetInputMode_GameOnly` _returnvalue)
  (set `PlayerController.bShowMouseCursor` false _returnvalue))

(fn `RecreateWeapon`
  (bind _weapon (`self.Weapon`))
  (`/Engine/EditorBlueprintResources/StandardMacros.IsValid` _weapon
    (:`Is Valid`
      (`Weapon.Destroy` _weapon))
    (:`Is Not Valid`
      _))
  (bind _returnvalue (`|GenericCreateObject` "/Game/Blueprints/Weapon/M4/M4.M4_C" (`GameplayStatics.GetPlayerController` 0)))
  (`Weapon.OnEquipped` _returnvalue (`self.Gun`))
  (set `self.Weapon` _returnvalue))

(fn `Save`
  (bind _asbase_character (cast `BaseCharacter` (`GameplayStatics.GetPlayerCharacter` 0)))
  (bind _returnvalue (`Weapon.Clone` (`self.Weapon`)))
  (`BaseCharacter.EquipWeapon` _asbase_character _returnvalue)
  (`self.Quit`))

(fn `UserConstructionScript`)